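; BP_Camera is a testing Blueprint that sets up the WBP_SystemControl user interface when play begins.
; It creates the widget, stores it, adds it to the viewport, then switches player 0 to UI-only input with a visible mouse cursor.
; It then finds the BP_Spawner in the level and, if one exists, passes it the widget through WidgetSpawned.
; Despite the name, its graphs contain no camera logic.
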(event `self.ReceiveBeginPlay`
  (bind _returnvalue (`GameplayStatics.GetPlayerController` 0))
  (bind _returnvalue_2 (`|CreateWidget` "/Game/Blueprints/Testing/Widget/WBP_SystemControl.WBP_SystemControl_C"))
  (bind _output_get (set `self.Widget` _returnvalue_2))
  (`UserWidget.AddToViewport` _output_get 0)
  (`WidgetBlueprintLibrary.SetInputMode_UIOnlyEx` _returnvalue (`self.Widget`))
  (set `PlayerController.bShowMouseCursor` true _returnvalue)
  (bind _returnvalue_3 (`GameplayStatics.GetActorOfClass` "/Game/Blueprints/Testing/BP_Spawner.BP_Spawner_C"))
  (`/Engine/EditorBlueprintResources/StandardMacros.IsValid` _returnvalue_3
    (:`Is Valid`
      (`/Game/Blueprints/Testing/Interfaces/BPI_Spawner.WidgetSpawned` _returnvalue_3 (`self.Widget`)))))

(fn `UserConstructionScript`)