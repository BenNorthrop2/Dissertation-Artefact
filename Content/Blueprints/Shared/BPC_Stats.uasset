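; Actor component that tracks Thirst, Hunger and Energy for its owner and queues whichever needs run low.
; Stats start at random values, and a looping timer drains them through a clamping macro, then broadcasts HandleUpdateStats.
; Stats below a quarter of maximum join the unique Needs list in detection order, readable by index through GetLowestNeeds.
; RefillStats adds a clamped amount and removes that need from the list.
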(event `self.ReceiveBeginPlay`
  (set `self.Stats` (make `/Game/Blueprints/Shared/Data/F_Stats` (`KismetMathLibrary.RandomFloatInRange` 50.0 100.0) (`KismetMathLibrary.RandomFloatInRange` 50.0 100.0) (`KismetMathLibrary.RandomFloatInRange` 50.0 100.0)))
  (`KismetSystemLibrary.K2_SetTimerDelegate` (`|CreateDelegate` :!event `DecreaseStats`) 1.0 true))

(event `DecreaseStats`
  (bind (_thirst _hunger _energy) (break `/Game/Blueprints/Shared/Data/F_Stats` (`self.MaxStats`)))
  (bind (_thirst_2 _hunger_2 _energy_2) (break `/Game/Blueprints/Shared/Data/F_Stats` (`self.Stats`)))
  (bind _currentvalueout (`self.SubtractStatValues` _thirst_2 _thirst)
    (:`Output`
      (setmembers `/Game/Blueprints/Shared/Data/F_Stats` :`StructRef` (`self.Stats`) :`Thirst` _currentvalueout)
      (bind _currentvalueout_2 (`self.SubtractStatValues` _hunger_2 _hunger "NewEnumerator1")
        (:`Output`
          (setmembers `/Game/Blueprints/Shared/Data/F_Stats` :`StructRef` (`self.Stats`) :`Hunger` _currentvalueout_2)
          (bind _currentvalueout_3 (`self.SubtractStatValues` _energy_2 _energy "NewEnumerator2")
            (:`Output`
              (setmembers `/Game/Blueprints/Shared/Data/F_Stats` :`StructRef` (`self.Stats`) :`Energy` _currentvalueout_3)
              (`self.HandleUpdateStats`))))))))

(event `DebugValues`
  ;[0.5781 0.5253 0.001657 0.5] Debug
  (`KismetSystemLibrary.PrintString` (`KismetTextLibrary.Conv_TextToString` (`|FormatText` "Owner: {A} \nThirst: {T} \nHunger: {H} \nEnergy: {E}" (`self.GetOwner`) _ _ _))))

(fn `GetLowestNeeds`
  (params (Index :type Integer))
  (returns (LowestNeedType :type "/Game/Blueprints/Shared/Data/E_NeedType Enum") (IsNeeded :type Boolean))
  (locals (LowestStat :type "Float (double-precision)" :default 100.0) (OutNeed :type "/Game/Blueprints/Shared/Data/E_NeedType Enum"))
  (if (`KismetArrayLibrary.Array_IsValidIndex` (`self.Needs`) Index)
    (return (`|GetArrayItem` (`self.Needs`) (`local.Index`)) true)
    (else
      (return "NewEnumerator3" false))))

(fn `RefillStats`
  (params (RefillAmount :type "Float (double-precision)") (StatType :type "/Game/Blueprints/Shared/Data/E_NeedType Enum" :default "NewEnumerator0"))
  (switch `/Game/Blueprints/Shared/Data/E_NeedType` StatType
    (:`NewEnumerator0`
      (setmembers `/Game/Blueprints/Shared/Data/F_Stats` :`StructRef` (`self.Stats`) :`Thirst` (`KismetMathLibrary.FClamp` (+ (`.Thirst_9_6F63E2A54ECFBE116AD40D899D3A1CA6` (break `/Game/Blueprints/Shared/Data/F_Stats` (`self.Stats`))) (`local.RefillAmount`)) 0.0 (`.Thirst_9_6F63E2A54ECFBE116AD40D899D3A1CA6` (break `/Game/Blueprints/Shared/Data/F_Stats` (`self.MaxStats`))))))
    (:`NewEnumerator1`
      (setmembers `/Game/Blueprints/Shared/Data/F_Stats` :`StructRef` (`self.Stats`) :`Hunger` (`KismetMathLibrary.FClamp` (+ (`.Hunger_10_5EF965FB4478089AE255918986110572` (break `/Game/Blueprints/Shared/Data/F_Stats` (`self.Stats`))) (`local.RefillAmount`)) 0.0 (`.Hunger_10_5EF965FB4478089AE255918986110572` (break `/Game/Blueprints/Shared/Data/F_Stats` (`self.MaxStats`))))))
    (:`NewEnumerator2`
      (setmembers `/Game/Blueprints/Shared/Data/F_Stats` :`StructRef` (`self.Stats`) :`Energy` (`KismetMathLibrary.FClamp` (+ (`.Energy_11_2E1B2BDE4CCB695D276D72A61AA32CB3` (break `/Game/Blueprints/Shared/Data/F_Stats` (`self.Stats`))) (`local.RefillAmount`)) 0.0 (`.Energy_11_2E1B2BDE4CCB695D276D72A61AA32CB3` (break `/Game/Blueprints/Shared/Data/F_Stats` (`self.MaxStats`)))))))
  (`KismetArrayLibrary.Array_RemoveItem` (`self.Needs`) (`local.StatType`)))

(fn `ReportLowStat`
  (params (Need :type "/Game/Blueprints/Shared/Data/E_NeedType Enum" :default "NewEnumerator0"))
  (`KismetArrayLibrary.Array_AddUnique` (`self.Needs`) Need))