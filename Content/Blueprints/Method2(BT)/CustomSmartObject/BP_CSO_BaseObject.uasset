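; BP_CSO_BaseObject is a custom smart object base that characters can claim and use to refill a need.
; A simple IsOccupied flag acts as the reservation: TryClaimObject sets it and fails if already taken, and ReleaseObject clears it.
; GetInteractionInfo reports occupancy, stat type and the InteractionPoint location, while UseObject returns the refill amount, need type, animation montage and facing rotation for the caller to apply.
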(event `/Game/Blueprints/Method2(BT)/Interfaces/BPI_CustomInteraction.ReleaseObject`
  (set `self.IsOccupied` false))

(fn `GetInteractionInfo`
  (returns (IsOccupied :type Boolean) (InteractLocation :type "Vector Structure") (StatType :type "/Game/Blueprints/Shared/Data/E_NeedType Enum"))
  (return (`self.IsOccupied`) (`SceneComponent.K2_GetComponentLocation` (`self.InteractionPoint`)) (`self.StatType`)))

(fn `TryClaimObject`
  (params (User :type "Actor Object Reference"))
  (returns (Success :type Boolean))
  (if (`self.IsOccupied`)
    (return false)
    (else
      (set `self.IsOccupied` true)
      (return true))))

(fn `UseObject`
  (returns (`Refill Amount` :type "Float (double-precision)") (NeedType :type "/Game/Blueprints/Shared/Data/E_NeedType Enum") (`Interaction Anim Montage` :type "AnimMontage Object Reference") (InteractRotation :type "Rotator Structure"))
  (return (`self.RefillAmount`) (`self.StatType`) (`self.InteractionMontage`) (`SceneComponent.K2_GetComponentRotation` (`self.InteractionPoint`))))

(fn `UserConstructionScript`)