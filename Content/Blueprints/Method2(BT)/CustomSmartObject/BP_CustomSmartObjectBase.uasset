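; Base custom smart object that actors claim and use to refill a need type.
; It reports occupancy, interaction location, need type and current user, and its use function returns refill amount, need and animation montage.
; SetOccupied acts as a claim check, failing when the requested state is already set, while ClearOccupied releases the user.
; A text render shows state for debugging, refreshed on construction, begin play and occupancy changes.
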(event `self.ReceiveBeginPlay`
  (`self.DebugText`))

(event `/Game/Blueprints/Method2(BT)/CustomSmartObject/Interfaces/BPI_CustomSOInteraction.ClearOccupied`
  (set `self.IsOccupied` false)
  (set `self.CurrentActor` null)
  (`self.DebugText`)
  (`KismetSystemLibrary.PrintString` "Hello"))

(fn `DebugText`
  (`TextRenderComponent.K2_SetText` (`self.TextRender`) (`|FormatText` "IsOccupied: {B} \nOwned Actor: {A} \nStat Type: {S}" (`self.IsOccupied`) (`KismetStringLibrary.GetSubstring` (`KismetSystemLibrary.GetDisplayName` (`self.CurrentActor`)) 0 15) (`|GetEnumeratorNameAsString` (`self.NeedType`)))))

(fn `GetInteractionInfo`
  (returns (IsOccupied :type Boolean) (InteractLocation :type "Vector Structure") (StatType :type "/Game/Blueprints/Shared/Data/E_NeedType Enum") (CurrentUser :type "Actor Object Reference"))
  (return (`self.IsOccupied`) (`SceneComponent.K2_GetComponentLocation` (`self.InteractionLocation`)) (`self.NeedType`) (`self.CurrentActor`)))

(fn `SetOccupied`
  (params (IsClaimed :type Boolean) (OwningActor :type "Actor Object Reference"))
  (returns (Success :type Boolean))
  (if (== (`self.IsOccupied`) IsClaimed)
    (return false)
    (else
      (set `self.IsOccupied` (`local.IsClaimed`))
      (set `self.CurrentActor` (`local.OwningActor`))
      (`self.DebugText`)
      (return true))))

(fn `UseObject`
  (returns (`Refill Amount` :type "Float (double-precision)") (NeedType :type "/Game/Blueprints/Shared/Data/E_NeedType Enum") (`Interaction Anim Montage` :type "AnimMontage Object Reference"))
  (return (`self.RefillAmount`) (`self.NeedType`) (`self.InteractionAnimationMontage`)))

(fn `UserConstructionScript`
  (`self.DebugText`))