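; BP_BT_AIChar is the AI character Blueprint for the behavior tree agent method, holding its needs stats.
; Its construction script assigns AIC_BT_Char as the AI controller class.
; A BPCStats component stores the needs; RefillStatsValues forwards a need type and amount to its RefillStats.
; GetNeeds and GetSkeletalMesh expose the component's needs and the character mesh.
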(event `/Game/Blueprints/Shared/Interfaces/BPI_StatsInterface.RefillStatsValues`
  (params (RefillAmount :type "Float (double-precision)") (NeedType :type "/Game/Blueprints/Shared/Data/E_NeedType Enum" :default "NewEnumerator3"))
  (`/Game/Blueprints/Shared/BPC_Stats.RefillStats` (`self.BPC_Stats`) RefillAmount NeedType))

(fn `GetNeeds`
  (returns (LowestNeed :type "Array of /Game/Blueprints/Shared/Data/E_NeedType Enum"))
  (return (`/Game/Blueprints/Shared/BPC_Stats.Needs` (`self.BPC_Stats`))))

(fn `GetSkeletalMesh`
  (returns (SkeletalMesh :type "SkeletalMeshComponent Object Reference"))
  (return (`self.Mesh`)))

(fn `UserConstructionScript`
  (set `self.AIControllerClass` "/Game/Blueprints/Method2(BT)/AIC_BT_Char.AIC_BT_Char_C"))