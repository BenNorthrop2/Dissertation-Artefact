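; BP_ST_AIChar is an AI agent character with needs stats, paired with the AIC_ST_Char controller.
; It delegates stats to its BPCStats component, forwarding refill requests by need type and exposing the component's Needs through GetNeeds.
; It sets AIControllerClass one tick after BeginPlay and again on landing, with no explicit controller spawn or possession in its graphs.
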(event `self.ReceiveBeginPlay`
  (`KismetSystemLibrary.DelayUntilNextTick`)
  (set `self.AIControllerClass` "/Game/Blueprints/Method1(ST)/AIC_ST_Char.AIC_ST_Char_C"))

(event `/Game/Blueprints/Shared/Interfaces/BPI_StatsInterface.RefillStatsValues`
  (params (RefillAmount :type "Float (double-precision)") (NeedType :type "/Game/Blueprints/Shared/Data/E_NeedType Enum" :default "NewEnumerator3"))
  (`/Game/Blueprints/Shared/BPC_Stats.RefillStats` (`self.BPC_Stats`) RefillAmount NeedType))

(event `self.OnLanded`
  (params (Hit :type "HitResult Structure (by ref)"))
  (set `self.AIControllerClass` "/Game/Blueprints/Method1(ST)/AIC_ST_Char.AIC_ST_Char_C"))

(fn `GetNeeds`
  (returns (LowestNeed :type "Array of /Game/Blueprints/Shared/Data/E_NeedType Enum"))
  (return (`/Game/Blueprints/Shared/BPC_Stats.Needs` (`self.BPC_Stats`))))

(fn `UserConstructionScript`)